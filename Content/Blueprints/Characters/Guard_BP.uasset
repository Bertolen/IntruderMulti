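; Guard character Blueprint that gives the guard a blue body color on both its Mesh and Mesh1P components.
; The Construction Script creates a dynamic material instance from slot 0 of each mesh and sets its BodyColor parameter.
; The event graph holds only disabled default events, so this Blueprint adds no runtime logic of its own.
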(fn `UserConstructionScript`
  (bind _mesh (`self.Mesh`))
  (bind _mesh1p (`self.Mesh1P`))
  (bind _returnvalue (`PrimitiveComponent.CreateDynamicMaterialInstance` _mesh 0 (`|GetArrayItem` (`MeshComponent.GetMaterials` _mesh))))
  (`MaterialInstanceDynamic.SetVectorParameterValue` _returnvalue "BodyColor" (make `LinearColor` 0.0 0.0 1.0))
  (bind _returnvalue_2 (`PrimitiveComponent.CreateDynamicMaterialInstance` _mesh1p 0 (`|GetArrayItem` (`MeshComponent.GetMaterials` _mesh1p))))
  (`MaterialInstanceDynamic.SetVectorParameterValue` _returnvalue_2 "BodyColor" (make `LinearColor` 0.0 0.0 1.0)))