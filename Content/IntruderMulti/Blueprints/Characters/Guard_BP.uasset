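; Guard character Blueprint for IntruderMulti that tints the guard's body.
; The construction script creates dynamic material instances on the first material slot of both Mesh and the first-person Mesh1P.
; It sets BodyColor on each to a dark maroon, through a color select hardwired to that choice.
; The event graph holds only disabled placeholder events, so this graph adds no runtime logic.
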(fn `UserConstructionScript`
  (bind _returnvalue (`KismetMathLibrary.SelectColor` (struct :`R` 0.322917 :`G` 0.095275 :`B` 0.167249 :`A` 1.0) (struct) true))
  (bind _mesh (`self.Mesh`))
  (bind _mesh1p (`self.Mesh1P`))
  (bind _returnvalue_2 (`PrimitiveComponent.CreateDynamicMaterialInstance` _mesh 0 (`|GetArrayItem` (`MeshComponent.GetMaterials` _mesh)) "None"))
  (`MaterialInstanceDynamic.SetVectorParameterValue` _returnvalue_2 "BodyColor" _returnvalue)
  (bind _returnvalue_3 (`PrimitiveComponent.CreateDynamicMaterialInstance` _mesh1p 0 (`|GetArrayItem` (`MeshComponent.GetMaterials` _mesh1p)) "None"))
  (`MaterialInstanceDynamic.SetVectorParameterValue` _returnvalue_3 "BodyColor" _returnvalue))