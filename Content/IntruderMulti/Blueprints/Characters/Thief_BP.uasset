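; Thief character Blueprint that tints its body to show whether it is carrying a valuable.
; The construction script creates a dynamic material instance from the mesh's first material and sets its initial BodyColor.
; Tick reapplies BodyColor every frame, choosing between the carrier and thief colors from IsCarryingAValuable.
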(event `self.ReceiveTick`
  (params (DeltaSeconds :type "Float (single-precision)"))
  (`MaterialInstanceDynamic.SetVectorParameterValue` (`self.MaterialInstance`) "BodyColor" (`KismetMathLibrary.SelectColor` (`self.CarrierColor`) (`self.ThiefColor`) (`self.bIsCarryingAValuable`))))

(fn `UserConstructionScript`
  (bind _mesh (`self.Mesh`))
  (bind _returnvalue (`PrimitiveComponent.CreateDynamicMaterialInstance` _mesh 0 (`|GetArrayItem` (`MeshComponent.GetMaterials` _mesh)) "None"))
  (bind _output_get (set `self.MaterialInstance` _returnvalue))
  (`MaterialInstanceDynamic.SetVectorParameterValue` _output_get "BodyColor" (`KismetMathLibrary.SelectColor` (`self.CarrierColor`) (`self.ThiefColor`) (`self.bIsCarryingAValuable`))))